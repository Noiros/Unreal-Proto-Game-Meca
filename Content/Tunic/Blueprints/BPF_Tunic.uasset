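; Blueprint function library for the Tunic game folder, with helpers for matching directional input sequences.
; VecToDir maps the four exact unit axis vectors to direction enum values, with no explicit result for other inputs.
; ValidateInputBuffer trims the oldest entries from a working copy of the buffer until it is no longer than the valid sequence, then returns whether both arrays are identical.
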(fn VectoDir
  (params (Input :type Vector%202D%20Structure))
  ;[1 1 1] Transforme l'input en direction
  (Utilities|FlowControl|Sequence
    (:then_0
      (if (Class|KismetMathLibrary|EqualExactlyVector2DVector2D Input "(X=1.000000,Y=0.000000)")
        (return "NewEnumerator3")))
    (:then_1
      (if (Class|KismetMathLibrary|EqualExactlyVector2DVector2D Input "(X=-1.000000,Y=0.000000)")
        (return "NewEnumerator2")))
    (:then_2
      (if (Class|KismetMathLibrary|EqualExactlyVector2DVector2D Input "(X=0.000000,Y=1.000000)")
        (return "NewEnumerator0")))
    (:then_3
      (if (Class|KismetMathLibrary|EqualExactlyVector2DVector2D Input "(X=0.000000,Y=-1.000000)")
        (return "NewEnumerator1")))))

(fn ValidateInputBuffer
  (params (Valid%20Sequence :type Array%20of%20E_Directions%20Enums :default "NewEnumerator0") (Input%20Buffer :type Array%20of%20E_Directions%20Enums :default "NewEnumerator0"))
  ;[1 1 1] Vérifie si l'input buffer est valide
  (bind _output_get (LocalVariables|SetTmp%20Input%20Buffer Input%20Buffer))
  (while (> (Utilities|Array|Length _output_get) (Utilities|Array|Length Valid%20Sequence))
    (Utilities|Array|RemoveIndex (LocalVariables|GetTmp%20Input%20Buffer)))
  (if (Utilities|Array|Identical (LocalVariables|GetTmp%20Input%20Buffer) Valid%20Sequence)
    (return true)
    (else
      (return false))))