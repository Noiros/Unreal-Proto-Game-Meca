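; BP_Cross is a directional-code lock, referenced as a door by BP_TunicCharacter, that opens when a set sequence of inputs is entered.
; BeginPlay converts the InputSeq directions into 2D vectors, and the sphere overlap sets or clears the character's DoorRef.
; CrossPressed appends each input vector and compares it with the target, clearing progress on a mismatch.
; A full match sets IsOpen and calls Triggered, which is empty here.
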(event OnComponentBeginOverlap(Sphere)
  (params (OverlappedComponent :type Primitive%20Component%20Object%20Reference) (OtherActor :type Actor%20Object%20Reference) (OtherComp :type Primitive%20Component%20Object%20Reference) (OtherBodyIndex :type Integer) (bFromSweep :type Boolean) (SweepResult :type Hit%20Result%20Structure%20%28by%20ref%29))
  (bind _asbp_tunic_character (Utilities|Casting|CastToBP_TunicCharacter OtherActor))
  (Variables|/Game/Tunic/BP_TunicCharacter.BP_TunicCharacter_C|SetDoorRef _asbp_tunic_character self))

(event OnComponentEndOverlap(Sphere)
  (params (OverlappedComponent :type Primitive%20Component%20Object%20Reference) (OtherActor :type Actor%20Object%20Reference) (OtherComp :type Primitive%20Component%20Object%20Reference) (OtherBodyIndex :type Integer))
  (bind _asbp_tunic_character (Utilities|Casting|CastToBP_TunicCharacter OtherActor))
  (Variables|/Game/Tunic/BP_TunicCharacter.BP_TunicCharacter_C|SetDoorRef _asbp_tunic_character 0))

(event Custom|CrossPressed
  (params (Vect :type Vector%202D%20Structure))
  (if (not (Variables|Default|GetIsOpen))
    (Utilities|Array|Add (Variables|Default|GetCurrentInputSeq) Vect)
    (if (Utilities|Array|Identical (Variables|Default|GetCurrentInputSeq) (Variables|Default|GetValidInputSeq))
      (Development|PrintString "OPEN")
      (Variables|Default|SetIsOpen true)
      (CallFunction|Triggered)
      (else
        (for (_array_element _array_index) (Variables|Default|GetCurrentInputSeq)
          (if (Utilities|Operators|NotEqual(!=) _array_element (Utilities|Array|Get(acopy) (Variables|Default|GetValidInputSeq) _array_index) 0.1)
            (Utilities|Array|Clear (Variables|Default|GetCurrentInputSeq))
            (Development|PrintString "RESET")))))))

(event Custom|Triggered)

(event EventBeginPlay
  (bind _validinputseq (Variables|Default|GetValidInputSeq))
  (for _array_element (Variables|Default|GetInputSeq)
    (switch Utilities|FlowControl|Switch|SwitchonE_Directions _array_element
      (:NewEnumerator0
        (Utilities|Array|Add _validinputseq "(X=0.000000,Y=1.000000)"))
      (:NewEnumerator1
        (Utilities|Array|Add _validinputseq "(X=0.000000,Y=-1.000000)"))
      (:NewEnumerator2
        (Utilities|Array|Add _validinputseq "(X=-1.000000,Y=0.000000)"))
      (:NewEnumerator3
        (Utilities|Array|Add _validinputseq "(X=1.000000,Y=0.000000)")))))

(fn ConstructionScript)