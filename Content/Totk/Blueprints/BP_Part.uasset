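; BP_Part is a physics part with attach points, apparently for a build-by-attaching mechanic.
; On BeginPlay it registers its Box as the physics object, collects the sphere components under Attach into AttachPoints, and resets the PhysicsHandle target to the origin.
; Unconnected logic throws the item, teleports it by the offset between two world locations and tells BP_Master to update parts, but never runs.
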(event EventBeginPlay
  (Variables|New|SetPhysicObject (Variables|Default|GetBox))
  (for _array_element (Components|GetChildrenComponents (Variables|Default|GetAttach) false)
    (bind _assphere_collision (Utilities|Casting|CastToSphereComponent _array_element))
    (Utilities|Array|Add (Variables|New|GetAttachPoints) _assphere_collision)
    (Physics|Components|PhysicsHandle|SetTargetLocation (Variables|Default|GetPhysicsHandle) "0, 0, 0")))

(fn ConstructionScript)