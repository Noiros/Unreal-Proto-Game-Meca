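; Manager actor that joins BP_Part actors in the level through spawned BP_Attachments constraint actors.
; BeginPlay gathers all parts and runs UpdateParts, which clears old joints and compares children of each part's Attach component pairwise.
; Points within a small distance spawn an attachment midway between the two actors to link them; each ordered pair is tested separately.
; Clearing, also run on EndPlay, destroys only the stored attachments' constraint components.
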(event Custom|UpdateParts
  (bind _partsref (Variables|Default|GetPartsRef))
  (CallFunction|ClearAttachments)
  (for _array_element _partsref
    (for _array_element_2 _partsref
      (if (!= _array_element_2 _array_element)
        (bind _array_element_3 (Utilities|Array|ForEachLoopwithBreak (Components|GetChildrenComponents (Variables|/Game/Totk/Blueprints/BP_Part.BP_Part_C|GetAttach _array_element_2) false) :!label _label)
          (:LoopBody
            (bind _array_element_4 (Utilities|Array|ForEachLoopwithBreak (Components|GetChildrenComponents (Variables|/Game/Totk/Blueprints/BP_Part.BP_Part_C|GetAttach _array_element) false))
              (:LoopBody
                (if (< (Math|Vector|Distance(Vector) (Transformation|GetWorldLocation _array_element_4) (Transformation|GetWorldLocation _array_element_3)) 5e+01)
                  (Utilities|FlowControl|Sequence
                    (:then_0
                      (bind _returnvalue (Game|SpawnActorfromClass "/Game/Totk/Blueprints/BP_Attachments.BP_Attachments_C" (Math|Conversions|ToTransform(Vector) (Math|Vector|Lerp(Vector) (Transformation|GetActorLocation _array_element_2) (Transformation|GetActorLocation _array_element) 0.5)) "Undefined" "MultiplyWithRoot" 0 0))
                      (Utilities|Array|AddUnique (Variables|Default|GetConstrains) _returnvalue)
                      (Default|Attach _returnvalue _array_element _array_element_2))
                    (:then_1
                      (goto _label Break))))))))))))

(event Custom|Clear%20Attachments
  (for _array_element (Variables|Default|GetConstrains)
    (Utilities|IsValid _array_element
      (:Is%20Valid
        (Components|DestroyComponent (Variables|/Script/Engine.PhysicsConstraintActor|GetConstraintComp _array_element))))))

(event EventBeginPlay
  (bind _outactors (Actor|GetAllActorsOfClass "/Game/Totk/Blueprints/BP_Part.BP_Part_C"))
  (Variables|Default|SetPartsRef _outactors)
  (CallFunction|UpdateParts))

(event EventEndPlay
  (params (EndPlayReason :type EEndPlayReason%20Enum :default "Destroyed"))
  (for _array_element (Variables|Default|GetConstrains)
    (Utilities|IsValid _array_element
      (:Is%20Valid
        (Components|DestroyComponent (Variables|/Script/Engine.PhysicsConstraintActor|GetConstraintComp _array_element))))))

(fn ConstructionScript)