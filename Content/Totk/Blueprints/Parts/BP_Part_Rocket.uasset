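; BP_Part_Rocket is a rocket part that propels itself along its up axis while active, then destroys itself.
; The ActiveObjects event sets the active flag that gates all Tick logic.
; Each active Tick adds delta-scaled linear velocity to the physics Box along its up vector and counts down LifeTime.
; Parent Tick runs only while the rocket is active and has not expired.
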(event EventBeginPlay)

(event Collision|EventActorBeginOverlap
  (params (OtherActor :type Actor%20Object%20Reference)))

(event EventTick
  (params (DeltaSeconds :type Float%20%28single-precision%29))
  (if (Variables|Default|GetIs%20Active)
    (Physics|SetPhysicsLinearVelocity (Variables|Default|GetBox) (* (* (Math|Vector|GetUpVector (Variables|Default|GetBox)) DeltaSeconds) 5e+03) true "None")
    (bind _output_get (Variables|Default|SetLifeTime (- (Variables|Default|GetLifeTime) DeltaSeconds)))
    (if (< _output_get 0.0)
      (Actor|DestroyActor)
      (else
        (|CallParentFunction DeltaSeconds)))))

(event EventActiveObjects
  (params (Active :type Boolean))
  (Variables|Default|SetIs%20Active Active))

(fn ConstructionScript
  (|CallParentFunction))