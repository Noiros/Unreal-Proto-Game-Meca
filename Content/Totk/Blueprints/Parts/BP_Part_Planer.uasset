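; BP_Part_Planer is a physics part that turns falling speed into horizontal motion, apparently as a glider.
; Each Tick it reads the Box's linear velocity and acts only while it moves downward.
; It then overwrites X and Y velocity with the actor's forward vector scaled by fall speed and Speed, leaving Z unchanged.
; The construction script only calls the parent's.
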(event EventBeginPlay)

(event Collision|EventActorBeginOverlap
  (params (OtherActor :type Actor%20Object%20Reference)))

(event EventTick
  (params (DeltaSeconds :type Float%20%28single-precision%29))
  (bind _returnvalue (Physics|GetPhysicsLinearVelocity (Variables|Default|GetBox) "None"))
  (if (< (.z _returnvalue) 0.0)
    (Physics|SetPhysicsLinearVelocity (Variables|Default|GetBox) (Math|Vector|MakeVector (.x (* (Transformation|GetActorForwardVector) (* (.z _returnvalue) (Variables|Default|GetSpeed)))) (.y (* (Transformation|GetActorForwardVector) (* (.z _returnvalue) (Variables|Default|GetSpeed)))) (.z _returnvalue)) false "None")))

(fn ConstructionScript
  (|CallParentFunction))