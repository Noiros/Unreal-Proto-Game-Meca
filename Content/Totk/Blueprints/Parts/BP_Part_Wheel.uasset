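; BP_Part_Wheel is a wheel part that drives itself forward while switched on.
; The ActiveObjects event stores its Active argument in IsActive.
; While that flag is set, Tick overwrites the Box's physics linear velocity with a fixed speed along its forward vector, replacing any existing velocity, gravity's included.
; The parent Tick runs only in that active branch.
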(event EventBeginPlay)

(event Collision|EventActorBeginOverlap
  (params (OtherActor :type Actor%20Object%20Reference)))

(event EventTick
  (params (DeltaSeconds :type Float%20%28single-precision%29))
  (if (Variables|Default|GetIs%20Active)
    (Physics|SetPhysicsLinearVelocity (Variables|Default|GetBox) (* (Math|Vector|GetForwardVector (Variables|Default|GetBox)) 100) false "None")
    (|CallParentFunction 0.0)))

(event EventActiveObjects
  (params (Active :type Boolean))
  (Variables|Default|SetIs%20Active Active))

(fn ConstructionScript
  (|CallParentFunction))