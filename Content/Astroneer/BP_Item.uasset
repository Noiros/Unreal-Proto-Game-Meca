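; Grabbable physics item that the player drags around with the mouse, throws, or attaches.
; Grabbing starts a looping near-frame-rate timer that steers the Box by linear velocity toward a point off the cursor's hit surface along its normal, while easing rotation to zero.
; Throwing stops the timer; attaching also stops it and disables physics simulation, leaving the passed Handler unused.
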(event Custom|GrabItem
  (if (not (Variables|Default|GetIsGrabbed))
    (bind _returnvalue (Actor|GetActorOfClass "/Game/Astroneer/BP_AstroCharacter.BP_AstroCharacter_C"))
    (Variables|Default|SetPlayerRef _returnvalue)
    (Variables|Default|SetIsGrabbed true)
    (bind _returnvalue_2 (Utilities|Time|SetTimerbyFunctionName 0 "ProcessDrag" 0.016 true true))
    (Variables|Default|SetTimer _returnvalue_2)))

(event Custom|ThrowItem
  (if (Variables|Default|GetIsGrabbed)
    (Variables|Default|SetIsGrabbed false)
    (Utilities|Time|ClearandInvalidateTimerbyHandle (Variables|Default|GetTimer))))

(event Custom|AttachItem
  (params (Handler :type BP%20Item%20Handler%20Object%20Reference))
  (Variables|Default|SetIsGrabbed false)
  (Physics|SetSimulatePhysics (Variables|Default|GetBox) false)
  (Utilities|Time|ClearandInvalidateTimerbyHandle (Variables|Default|GetTimer)))

(event Custom|ProcessDrag
  (bind (_result _normal) (Default|GetMousePosition (Variables|Default|GetPlayerRef) 5e+03 (Utilities|Array|MakeArray self)))
  (Physics|SetPhysicsLinearVelocity (Variables|Default|GetBox) (* (- (+ _result (* _normal 1e+02)) (Transformation|GetActorLocation)) 1e+01) false "None")
  (Transformation|SetActorRotation (Math|Rotator|Lerp(Rotator) (Transformation|GetActorRotation) "0, 0, 0" 0.2)))

(fn ConstructionScript)