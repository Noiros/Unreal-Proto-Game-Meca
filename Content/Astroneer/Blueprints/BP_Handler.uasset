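; BP_Handler is an Astroneer-style attachment slot that snaps a grabbed BP_Object of matching size onto itself.
; When a valid object overlaps its empty sphere, a fast looping timer teleports it to the Scene component's transform and registers the handler as its NearHandler.
; Moving the object too fast clears that link and the timer, while ending overlap clears only the timer.
; AttachObject and UnAttachObject set or clear the held object and fire UpdateItem.
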(event OnComponentBeginOverlap(Sphere)
  (params (OverlappedComponent :type Primitive%20Component%20Object%20Reference) (OtherActor :type Actor%20Object%20Reference) (OtherComp :type Primitive%20Component%20Object%20Reference) (OtherBodyIndex :type Integer) (bFromSweep :type Boolean) (SweepResult :type Hit%20Result%20Structure%20%28by%20ref%29))
  (Utilities|IsValid (Variables|Default|GetObject)
    (:Is%20Not%20Valid
      (bind _asbp_object (Utilities|Casting|CastToBP_Object OtherActor))
      (bind _output_get (Variables|Default|SetDraggedObject _asbp_object))
      (if (and (Utilities|Enum|Equal(Enum) (Variables|/Game/Astroneer/Blueprints/BP_Object.BP_Object_C|GetSize _output_get) (Variables|Default|GetSize)) (Variables|/Game/Astroneer/Blueprints/BP_Object.BP_Object_C|GetIsGrabbed _asbp_object))
        (bind _returnvalue (Utilities|Time|SetTimerbyEvent (delegate Custom|ProcessAttach) 0.001 true true))
        (Variables|Default|SetTimer _returnvalue)))))

(event OnComponentEndOverlap(Sphere)
  (params (OverlappedComponent :type Primitive%20Component%20Object%20Reference) (OtherActor :type Actor%20Object%20Reference) (OtherComp :type Primitive%20Component%20Object%20Reference) (OtherBodyIndex :type Integer))
  (Utilities|Time|ClearandInvalidateTimerbyHandle (Variables|Default|GetTimer)))

(event Custom|ProcessAttach
  (bind _scene (Variables|Default|GetScene))
  (bind _draggedobject (Variables|Default|GetDraggedObject))
  (bind _returnvalue (Transformation|GetWorldTransform _scene))
  (bind (_location _rotation) (Math|Transform|BreakTransform _returnvalue))
  (if (< (Math|Vector|VectorLength (Transformation|GetVelocity _draggedobject)) 1e+03)
    (Transformation|SetActorTransform _draggedobject (Math|Transform|MakeTransform _location _rotation (.Scale (Math|Transform|BreakTransform (Transformation|GetRelativeTransform (Variables|/Game/Astroneer/Blueprints/BP_Object.BP_Object_C|GetAncorPoint _draggedobject))))) false true)
    (Variables|/Game/Astroneer/Blueprints/BP_Object.BP_Object_C|SetNearHandler _draggedobject self)
    (else
      (Utilities|Time|ClearandInvalidateTimerbyHandle (Variables|Default|GetTimer))
      (Variables|/Game/Astroneer/Blueprints/BP_Object.BP_Object_C|SetNearHandler _draggedobject 0))))

(event Custom|AttachObject
  (params (Object :type BP%20Object%20Object%20Reference))
  (Variables|Default|SetObject Object)
  (Default|CallUpdateItem))

(event Custom|UnAttachObject
  (Variables|Default|SetObject 0)
  (Default|CallUpdateItem))

(fn ConstructionScript)