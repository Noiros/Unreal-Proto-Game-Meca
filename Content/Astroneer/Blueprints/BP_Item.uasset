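; BP_Item is a data-driven item actor that shows a mesh and a name and description widget for its ItemMaterial.
; ItemMaterial, converted to a Name, selects the row in the Items data table.
; The construction script applies that row's static mesh to the Mesh component.
; On BeginPlay, the same lookup fills the title and description text of the WBP_ItemWidget held by the Widget component.
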(event EventBeginPlay
  (bind _returnvalue (Utilities|GetDataTableRow "/Game/Astroneer/Assets/Datas/Items.Items" (Utilities|String|StringToName (Variables|Default|GetItemMaterial)))
    (:then
      (bind _aswbp_item_widget (Utilities|Casting|CastToWBP_ItemWidget (UserInterface|GetWidget (Variables|Default|GetWidget))))
      (Rendering|Components|TextRender|SetText (Variables|/Game/Astroneer/Blueprints/WBP_ItemWidget.WBP_ItemWidget_C|GetTitle _aswbp_item_widget) (.ItemName (Utilities|Struct|BreakS_Items _returnvalue)))
      (Rendering|Components|TextRender|SetText (Variables|/Game/Astroneer/Blueprints/WBP_ItemWidget.WBP_ItemWidget_C|GetDesc _aswbp_item_widget) (.ItemDesc (Utilities|Struct|BreakS_Items _returnvalue))))))

(fn ConstructionScript
  (bind _returnvalue (Utilities|GetDataTableRow "/Game/Astroneer/Assets/Datas/Items.Items" (Utilities|String|StringToName (Variables|Default|GetItemMaterial)))
    (:then
      (Components|StaticMesh|SetStaticMesh (Variables|Default|GetMesh) (.Mesh (Utilities|Struct|BreakS_Items _returnvalue))))))