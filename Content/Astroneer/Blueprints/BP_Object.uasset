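; Grabbable physics object that the player drags with the mouse and docks into handlers, with a widget shown on hover.
; Grabbing detaches it from its handler and starts a looping timer that drives the box's velocity toward the cursor trace hit, offset along the surface normal, while easing rotation toward zero.
; Releasing stops the timer and, if a handler is near, disables physics and attaches to it.
; Interact is an empty stub.
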(event Custom|GrabObject
  (bind _handler (Variables|Default|GetHandler))
  (if (not (Variables|Default|GetIsGrabbed))
    (bind _returnvalue (Actor|GetActorOfClass "/Game/Astroneer/Blueprints/BP_AstroCharacter.BP_AstroCharacter_C"))
    (Variables|Default|SetPlayerRef _returnvalue)
    (Variables|Default|SetIsGrabbed true)
    (bind _returnvalue_2 (Utilities|Time|SetTimerbyFunctionName 0 "ProcessDrag" 0.016 true true))
    (Variables|Default|SetDragTimer _returnvalue_2)
    (Physics|SetSimulatePhysics (Variables|Default|GetBox) true)
    (Utilities|IsValid _handler
      (:Is%20Valid
        (Default|UnAttachObject _handler)))))

(event Custom|ThrowObject
  (bind _nearhandler (Variables|Default|GetNearHandler))
  (if (Variables|Default|GetIsGrabbed)
    (Variables|Default|SetIsGrabbed false)
    (Utilities|Time|ClearandInvalidateTimerbyHandle (Variables|Default|GetDragTimer))
    (Utilities|IsValid _nearhandler
      (:Is%20Valid
        (bind _output_get (Variables|Default|SetHandler _nearhandler))
        (CallFunction|AttachObject _output_get)))))

(event Custom|AttachObject
  (params (Handler :type BP%20Handler%20Object%20Reference))
  (Utilities|Time|ClearandInvalidateTimerbyHandle (Variables|Default|GetDragTimer))
  (Variables|Default|SetIsGrabbed false)
  (Physics|SetSimulatePhysics (Variables|Default|GetBox) false)
  (Default|AttachObject (Variables|Default|GetNearHandler) self))

(event Custom|ProcessDrag
  (bind (_result _normal) (Default|GetMousePosition (Variables|Default|GetPlayerRef) 5e+03 (Utilities|Array|MakeArray self) "TraceTypeQuery1"))
  (Physics|SetPhysicsLinearVelocity (Variables|Default|GetBox) (* (- (+ _result (* _normal 5e+01)) (Transformation|GetWorldLocation (Variables|Default|GetAncorPoint))) 1e+01) false "None")
  (Transformation|SetActorRotation (Math|Rotator|Lerp(Rotator) (Transformation|GetActorRotation) "0, 0, 0" 0.2 true)))

(event EventHover
  (Rendering|SetVisibility (Variables|Default|GetWidget) true false))

(event EventUnHover
  (Rendering|SetVisibility (Variables|Default|GetWidget) false false))

(event EventInteract)

(fn ConstructionScript)