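; Crafting printer building that turns items held in three child BP_Handler slots into an object defined by a recipe.
; BeginPlay creates a hidden WBP_Printer per handler, keeping the last in Widget, which Interact shows or hides.
; Choosing a recipe reads the PrinterCraft table, assigns requested items to handlers and drops held ones.
; Printing compares sorted held materials to the recipe, then spawns the result at SpawnPos and destroys the held items.
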(event Custom|Update%20Handler%20Item
  (params (Object :type BP%20Object%20Object%20Reference))
  (Development|PrintString (Utilities|GetDisplayName Object)))

(event Custom|Set%20Recipe
  (params (Name :type Name))
  (bind _output_get (Variables|Default|SetCurrent%20Object Name))
  (bind _returnvalue (Utilities|GetDataTableRow "/Game/Astroneer/Assets/Datas/PrinterCraft.PrinterCraft" _output_get)
    (:then
      (for (_array_element _array_index) (.itemneeded _returnvalue)
        (bind _asbp_handler (Utilities|Casting|CastToBP_Handler (Variables|/Script/Engine.ChildActorComponent|GetChildActor (Utilities|Array|Get(acopy) (Utilities|Array|MakeArray (Variables|Default|GetBP_Handler_1) (Variables|Default|GetBP_Handler_2) (Variables|Default|GetBP_Handler_3)) _array_index))))
        (Default|SetRequestItem _asbp_handler _array_element)
        (Utilities|IsValid (Variables|/Game/Astroneer/Blueprints/BP_Handler.BP_Handler_C|GetGrabbedItem _asbp_handler)
          (:Is%20Valid
            (Default|Drop (Variables|/Game/Astroneer/Blueprints/BP_Handler.BP_Handler_C|GetGrabbedItem _asbp_handler))))))))

(event Custom|Print%20Object
  (bind _has (CallFunction|HasItems))
  (if _has
    (bind _returnvalue (Utilities|GetDataTableRow "/Game/Astroneer/Assets/Datas/PrinterCraft.PrinterCraft" (Variables|Default|GetCurrent%20Object))
      (:then
        (Game|SpawnActorfromClass (.object _returnvalue) (Transformation|GetWorldTransform (Variables|Default|GetSpawn%20Pos)) "Undefined" "MultiplyWithRoot" 0 0)
        (for _array_element (Utilities|Array|MakeArray (Variables|Default|GetBP_Handler_1) (Variables|Default|GetBP_Handler_2) (Variables|Default|GetBP_Handler_3))
          (bind _asbp_handler (Utilities|Casting|CastToBP_Handler (Variables|/Script/Engine.ChildActorComponent|GetChildActor _array_element)))
          (Actor|DestroyActor (Variables|/Game/Astroneer/Blueprints/BP_Handler.BP_Handler_C|GetGrabbedItem _asbp_handler)))))))

(event EventInteract
  (bind _widget (Variables|Default|GetWidget))
  (switch Utilities|FlowControl|Switch|SwitchonESlateVisibility (Widget|GetVisibility _widget)
    (:Visible
      (Widget|SetVisibility _widget "Hidden"))
    (:Hidden
      (Widget|SetVisibility _widget "Visible"))))

(event EventBeginPlay
  (for _array_element (Utilities|Array|MakeArray (Variables|Default|GetBP_Handler_3) (Variables|Default|GetBP_Handler_2) (Variables|Default|GetBP_Handler_1))
    (bind _asbp_handler (Utilities|Casting|CastToBP_Handler (Variables|/Script/Engine.ChildActorComponent|GetChildActor _array_element)))
    (EventDispatchers|BindEventtoItemUpdated _asbp_handler (delegate Custom|Update%20Handler%20Item))
    (bind _returnvalue (UserInterface|CreateWidget "/Game/Astroneer/Blueprints/WBP_Printer.WBP_Printer_C" 0 self))
    (EventDispatchers|BindEventtoRecipeSet _returnvalue (delegate Custom|Set%20Recipe))
    (UserInterface|Viewport|AddtoViewport _returnvalue 0)
    (bind _output_get (Variables|Default|SetWidget _returnvalue))
    (Widget|SetVisibility _output_get "Hidden")
    (EventDispatchers|BindEventtoPrintObject _output_get (delegate Custom|Print%20Object))))

(fn ConstructionScript
  (|CallParentFunction))

(fn HasItems
  (bind _items (LocalVariables|GetItems))
  (for _array_element (Utilities|Array|MakeArray (Variables|Default|GetBP_Handler_1) (Variables|Default|GetBP_Handler_2) (Variables|Default|GetBP_Handler_3))
    (bind _asbp_handler (Utilities|Casting|CastToBP_Handler (Variables|/Script/Engine.ChildActorComponent|GetChildActor _array_element)))
    (Utilities|IsValid (Variables|/Game/Astroneer/Blueprints/BP_Handler.BP_Handler_C|GetGrabbedItem _asbp_handler)
      (:Is%20Valid
        (Utilities|Array|Add (LocalVariables|GetItems) (Utilities|String|StringToName (Variables|/Game/Astroneer/Blueprints/BP_Item.BP_Item_C|GetItemMaterial (Variables|/Game/Astroneer/Blueprints/BP_Handler.BP_Handler_C|GetGrabbedItem _asbp_handler)))))))
  (bind _returnvalue (Utilities|GetDataTableRow "/Game/Astroneer/Assets/Datas/PrinterCraft.PrinterCraft" (Variables|Default|GetCurrent%20Object))
    (:then
      (Class|KismetArrayLibrary|SortNameArray (.itemneeded _returnvalue))
      (Class|KismetArrayLibrary|SortNameArray _items)
      (return (Utilities|Array|Identical (.itemneeded _returnvalue) _items)))))