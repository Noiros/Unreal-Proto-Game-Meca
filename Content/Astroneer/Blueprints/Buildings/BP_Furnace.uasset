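; Furnace building that turns cookable items placed in its four input handlers into refined items.
; Input handler updates queue any item whose material has a row in the CookedItems data table.
; A timer processes the queue one item at a time, destroying the input when cooking starts.
; When the timer fires, the Result handler creates the table's refined item and the next queued item starts.
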(event Custom|Set%20Item
  (params (Object :type BP%20Object%20Object%20Reference))
  ;[1 1 1] Un item à été ajouté sur le handler, regarder si il est cuisable et si oui, l'ajouter dans la file d'attente
  (bind _asbp_item (Utilities|Casting|CastToBP_Item Object))
  (Utilities|GetDataTableRow "/Game/Astroneer/Assets/Datas/CookedItems.CookedItems" (Utilities|String|StringToName (Variables|/Game/Astroneer/Blueprints/BP_Item.BP_Item_C|GetItemMaterial _asbp_item))
    (:then
      (Utilities|Array|Add (Variables|Default|GetCookQueue) _asbp_item)
      (if (not (Utilities|Time|IsValidTimerHandle (Variables|Default|GetCookTimer)))
        (CallFunction|StartCook)))))

(event Custom|StartCook
  (bind _cookqueue (Variables|Default|GetCookQueue))
  (bind _output (Utilities|Array|Get(acopy) _cookqueue))
  ;[1 1 1] Retire l'item du slot et lance le timer de cuisson
  (bind _returnvalue (Utilities|Time|SetTimerbyEvent (delegate Custom|Cooked) (Variables|Default|GetCookDelay)))
  (Variables|Default|SetCookTimer _returnvalue)
  (Variables|Default|SetInCookItem (Utilities|String|StringToName (Variables|/Game/Astroneer/Blueprints/BP_Item.BP_Item_C|GetItemMaterial _output)))
  (Variables|/Game/Astroneer/Blueprints/BP_Handler.BP_Handler_C|SetGrabbedItem (Variables|/Game/Astroneer/Blueprints/BP_Object.BP_Object_C|GetHandler _output) 0)
  (Actor|DestroyActor _output)
  (Utilities|Array|RemoveIndex (Variables|Default|GetCookQueue)))

(event Custom|Cooked
  ;[1 1 1] Créer l'item de sortie et l'ajoute sur le handler
  (Utilities|Time|ClearandInvalidateTimerbyHandle (Variables|Default|GetCookTimer))
  (bind _asbp_handler (Utilities|Casting|CastToBP_Handler (Variables|/Script/Engine.ChildActorComponent|GetChildActor (Variables|Default|GetResult))))
  (bind _returnvalue (Utilities|GetDataTableRow "/Game/Astroneer/Assets/Datas/CookedItems.CookedItems" (Variables|Default|GetInCookItem))
    (:then
      (Default|CreateItem _asbp_handler (.refineitem _returnvalue))
      (if (not (Utilities|Array|IsEmpty (Variables|Default|GetCookQueue)))
        (CallFunction|StartCook)))))

(event EventBeginPlay
  ;[1 1 1] bind toutes les item updated des handler
  (for _array_element (Utilities|Array|MakeArray (Variables|Default|GetItem_1) (Variables|Default|GetItem_2) (Variables|Default|GetItem_3) (Variables|Default|GetItem_4))
    (bind _asbp_handler (Utilities|Casting|CastToBP_Handler (Variables|/Script/Engine.ChildActorComponent|GetChildActor _array_element)))
    (EventDispatchers|BindEventtoItemUpdated _asbp_handler (delegate Custom|Set%20Item))))

(fn ConstructionScript
  (|CallParentFunction))